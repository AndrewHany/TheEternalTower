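; Player character for The Eternal Tower, with inventory, equipment and combat stats.
; On BeginPlay the server initializes the inventory and spawns hardcoded test items into it, while remote instances link player controller 0's character widget and inventory UI.
; OnRepUpdate events refresh buffs, or equipment slots through a shared function setting icon, rarity frame and enhancement text.
; Stat getters return base plus bonus values.
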(event Custom|TestAdd
  (Networking|SwitchHasAuthority
    (:Authority
      (bind _returnvalue (Game|SpawnActorfromClass "/Game/Blueprints/Inventory/Items/BP_Item_E_Weapon_Absolution.BP_Item_E_Weapon_Absolution_C" (Math|Transform|MakeTransform "0, 0, 0") "Undefined" self 0))
      (Class|Inventory|AddItemtoInventory (Variables|Default|GetInventory) _returnvalue -1)
      (bind _returnvalue_2 (Game|SpawnActorfromClass "/Game/Blueprints/Inventory/Items/BP_Item_C_Potion_Experience.BP_Item_C_Potion_Experience_C" (Math|Transform|MakeTransform "0, 0, 0") "Undefined" self 100 0))
      (Class|Inventory|AddItemtoInventory (Variables|Default|GetInventory) _returnvalue_2 -1)
      (bind _returnvalue_3 (Game|SpawnActorfromClass "/Game/Blueprints/Inventory/Items/BP_Item_Ring_Serendipity.BP_Item_Ring_Serendipity_C" (Math|Transform|MakeTransform "0, 0, 0") "Undefined" self 0))
      (Class|Inventory|AddItemtoInventory (Variables|Default|GetInventory) _returnvalue_3 -1)
      (bind _returnvalue_4 (Game|SpawnActorfromClass "/Game/Blueprints/Inventory/Items/BP_Item_Ring_Serendipity.BP_Item_Ring_Serendipity_C" (Math|Transform|MakeTransform "0, 0, 0") "Undefined" self 0))
      (Class|Inventory|AddItemtoInventory (Variables|Default|GetInventory) _returnvalue_4 -1)
      (bind _returnvalue_5 (Game|SpawnActorfromClass "/Game/Blueprints/Inventory/Items/BP_Item_E_Armor_Juggernaut.BP_Item_E_Armor_Juggernaut_C" (Math|Transform|MakeTransform "0, 0, 0") "Undefined" self 0))
      (Class|Inventory|AddItemtoInventory (Variables|Default|GetInventory) _returnvalue_5 -1)
      (bind _returnvalue_6 (Game|SpawnActorfromClass "/Game/Blueprints/Inventory/Items/BP_Item_E_Armor_Demonrattler.BP_Item_E_Armor_Demonrattler_C" (Math|Transform|MakeTransform "0, 0, 0") "Undefined" self 0))
      (Class|Inventory|AddItemtoInventory (Variables|Default|GetInventory) _returnvalue_6 -1)
      (bind _returnvalue_7 (Game|SpawnActorfromClass "/Game/Blueprints/Inventory/Items/BP_Item_E_Armor_Angelwing.BP_Item_E_Armor_Angelwing_C" (Math|Transform|MakeTransform "0, 0, 0") "Undefined" self 0))
      (Class|Inventory|AddItemtoInventory (Variables|Default|GetInventory) _returnvalue_7 -1)
      (bind _returnvalue_8 (Game|SpawnActorfromClass "/Game/Blueprints/Inventory/Items/BP_Item_E_Weapon_Salvation.BP_Item_E_Weapon_Salvation_C" (Math|Transform|MakeTransform "0, 0, 0") "Undefined" self 0))
      (Class|Inventory|AddItemtoInventory (Variables|Default|GetInventory) _returnvalue_8 -1)
      (bind _returnvalue_9 (Game|SpawnActorfromClass "/Game/Blueprints/Inventory/Items/BP_Item_E_Weapon_SoulReaper.BP_Item_E_Weapon_SoulReaper_C" (Math|Transform|MakeTransform "0, 0, 0") "Undefined" self 0))
      (Class|Inventory|AddItemtoInventory (Variables|Default|GetInventory) _returnvalue_9 -1)
      (bind _returnvalue_10 (Game|SpawnActorfromClass "/Game/Blueprints/Inventory/Items/BP_Item_E_Weapon_Dragonslayer.BP_Item_E_Weapon_DragonSlayer_C" (Math|Transform|MakeTransform "0, 0, 0") "Undefined" self 0))
      (Class|Inventory|AddItemtoInventory (Variables|Default|GetInventory) _returnvalue_10 -1)
      (bind _returnvalue_11 (Game|SpawnActorfromClass "/Game/Blueprints/Inventory/Items/BP_Item_C_Potion_Death.BP_Item_C_Potion_Death_C" (Math|Transform|MakeTransform "0, 0, 0") "Undefined" self 10 0))
      (Class|Inventory|AddItemtoInventory (Variables|Default|GetInventory) _returnvalue_11 -1)
      (bind _returnvalue_12 (Game|SpawnActorfromClass "/Game/Blueprints/Inventory/Items/BP_Item_C_Potion_Divine.BP_Item_C_Potion_Divine_C" (Math|Transform|MakeTransform "0, 0, 0") "Undefined" self 20 0))
      (Class|Inventory|AddItemtoInventory (Variables|Default|GetInventory) _returnvalue_12 -1)
      (bind _returnvalue_13 (Game|SpawnActorfromClass "/Game/Blueprints/Inventory/Items/BP_Item_C_Potion_Health.BP_Item_C_Potion_Health_C" (Math|Transform|MakeTransform "0, 0, 0") "Undefined" self 200 0))
      (Class|Inventory|AddItemtoInventory (Variables|Default|GetInventory) _returnvalue_13 -1)
      (bind _returnvalue_14 (Game|SpawnActorfromClass "/Game/Blueprints/Inventory/Items/BP_Item_C_Potion_Mana.BP_Item_C_Potion_Mana_C" (Math|Transform|MakeTransform "0, 0, 0") "Undefined" self 200 0))
      (Class|Inventory|AddItemtoInventory (Variables|Default|GetInventory) _returnvalue_14 -1))))

(event EventBeginPlay
  (Networking|SwitchHasAuthority
    (:Authority
      (Class|Inventory|InitializeInventory (Variables|Default|GetInventory))
      (CallFunction|TestAdd))
    (:Remote
      (bind _asbp_the_eternal_tower_player_controller (Utilities|Casting|CastToBP_TheEternalTowerPlayerController (Game|GetPlayerController 0)))
      (bind _output_get (Variables|Default|SetMyPlayerController _asbp_the_eternal_tower_player_controller))
      (Variables|Default|SetCharacterWidget (Variables|/Script/TheEternalTower.TheEternalTowerPlayerController|GetMyCharacterWidget _output_get))
      (Default|InitInventory (Variables|Default|GetMyPlayerController) (Variables|Default|GetInventory)))))

(event EventOnRepUpdateRightEarring
  ;[0.5051 1 0.664] Updating Equipment Slots
  (bind _aswbp_character (Utilities|Casting|CastToWBP_Character (Variables|Default|GetCharacterWidget)))
  (CallFunction|UpdateEquipmentSlot (Variables|Default|GetRightEarring) (Variables|/Game/UI/WBP_Character.WBP_Character_C|GetRightEarringSlot _aswbp_character)))

(event EventOnRepUpdateLeftEarring
  ;[0.5051 1 0.664] Updating Equipment Slots
  (bind _aswbp_character (Utilities|Casting|CastToWBP_Character (Variables|Default|GetCharacterWidget)))
  (CallFunction|UpdateEquipmentSlot (Variables|Default|GetLeftEarring) (Variables|/Game/UI/WBP_Character.WBP_Character_C|GetLeftEarringSlot _aswbp_character)))

(event EventOnRepUpdateHelmet
  ;[0.5051 1 0.664] Updating Equipment Slots
  (bind _aswbp_character (Utilities|Casting|CastToWBP_Character (Variables|Default|GetCharacterWidget)))
  (CallFunction|UpdateEquipmentSlot (Variables|Default|GetHelmet) (Variables|/Game/UI/WBP_Character.WBP_Character_C|GetHelmetSlot _aswbp_character)))

(event EventOnRepUpdateNecklace
  ;[0.5051 1 0.664] Updating Equipment Slots
  (bind _aswbp_character (Utilities|Casting|CastToWBP_Character (Variables|Default|GetCharacterWidget)))
  (CallFunction|UpdateEquipmentSlot (Variables|Default|GetNecklace) (Variables|/Game/UI/WBP_Character.WBP_Character_C|GetNecklaceSlot _aswbp_character)))

(event EventOnRepUpdateArmor
  ;[0.5051 1 0.664] Updating Equipment Slots
  (bind _aswbp_character (Utilities|Casting|CastToWBP_Character (Variables|Default|GetCharacterWidget)))
  (CallFunction|UpdateEquipmentSlot (Variables|Default|GetArmor) (Variables|/Game/UI/WBP_Character.WBP_Character_C|GetArmorSlot _aswbp_character)))

(event EventOnRepUpdateLeftRing
  ;[0.5051 1 0.664] Updating Equipment Slots
  (bind _aswbp_character (Utilities|Casting|CastToWBP_Character (Variables|Default|GetCharacterWidget)))
  (CallFunction|UpdateEquipmentSlot (Variables|Default|GetLeftRing) (Variables|/Game/UI/WBP_Character.WBP_Character_C|GetLeftRingSlot _aswbp_character)))

(event EventOnRepUpdateRightRing
  ;[0.5051 1 0.664] Updating Equipment Slots
  (bind _aswbp_character (Utilities|Casting|CastToWBP_Character (Variables|Default|GetCharacterWidget)))
  (CallFunction|UpdateEquipmentSlot (Variables|Default|GetRightRing) (Variables|/Game/UI/WBP_Character.WBP_Character_C|GetRightRingSlot _aswbp_character)))

(event EventOnRepUpdateWeapon
  ;[0.5051 1 0.664] Updating Equipment Slots
  (bind _aswbp_character (Utilities|Casting|CastToWBP_Character (Variables|Default|GetCharacterWidget)))
  (CallFunction|UpdateEquipmentSlot (Variables|Default|GetWeapon) (Variables|/Game/UI/WBP_Character.WBP_Character_C|GetWeaponSlot _aswbp_character)))

(event EventOnRepUpdateGloves
  ;[0.5051 1 0.664] Updating Equipment Slots
  (bind _aswbp_character (Utilities|Casting|CastToWBP_Character (Variables|Default|GetCharacterWidget)))
  (CallFunction|UpdateEquipmentSlot (Variables|Default|GetGloves) (Variables|/Game/UI/WBP_Character.WBP_Character_C|GetGlovesSlot _aswbp_character)))

(event EventOnRepUpdateBoots
  ;[0.5051 1 0.664] Updating Equipment Slots
  (bind _aswbp_character (Utilities|Casting|CastToWBP_Character (Variables|Default|GetCharacterWidget)))
  (CallFunction|UpdateEquipmentSlot (Variables|Default|GetBoots) (Variables|/Game/UI/WBP_Character.WBP_Character_C|GetBootsSlot _aswbp_character)))

(event EventOnRepUpdateActiveBuffs
  (bind _asbp_the_eternal_tower_player_controller (Utilities|Casting|CastToBP_TheEternalTowerPlayerController (Game|GetPlayerController 0)))
  (Default|UpdateActiveBuffs _asbp_the_eternal_tower_player_controller))

(fn ConstructionScript)

(fn UpdateEquipmentSlot
  (params (Item :type Equippable%20Item%20Object%20Reference) (EquipmentSlot :type WBP%20Equipment%20Slot%20Object%20Reference))
  (LocalVariables|SetLocal%20Item Item)
  (LocalVariables|SetLocal%20EquipmentSlot EquipmentSlot)
  (Utilities|IsValid (LocalVariables|GetLocal%20Item)
    (:Is%20Valid
      (Variables|/Game/UI/WBP_EquipmentSlot.WBP_EquipmentSlot_C|SetHeld%20Item (LocalVariables|GetLocal%20EquipmentSlot) (LocalVariables|GetLocal%20Item))
      (Appearance|SetBrushfromTexture (Variables|/Game/UI/WBP_EquipmentSlot.WBP_EquipmentSlot_C|GetSlotIcon (LocalVariables|GetLocal%20EquipmentSlot)) (Variables|/Script/TheEternalTower.Item|GetItemIcon (LocalVariables|GetLocal%20Item)) false)
      (Widget|SetVisibility (Variables|/Game/UI/WBP_EquipmentSlot.WBP_EquipmentSlot_C|GetSlotIcon (LocalVariables|GetLocal%20EquipmentSlot)) "Visible")
      (Class|Image|SetOpacity (Variables|/Game/UI/WBP_EquipmentSlot.WBP_EquipmentSlot_C|GetSlotIcon (LocalVariables|GetLocal%20EquipmentSlot)) 1.0)
      (switch Utilities|FlowControl|Switch|SwitchonEItemRarity (Variables|/Script/TheEternalTower.Item|GetItemRarity (LocalVariables|GetLocal%20Item))
        (:RARITY_COMMON
          (Appearance|SetBrushfromTexture (Variables|/Game/UI/WBP_EquipmentSlot.WBP_EquipmentSlot_C|GetRarityIcon (LocalVariables|GetLocal%20EquipmentSlot)) "/Game/Textures/Inventory/T_ItemRarity_Common.T_ItemRarity_Common" false))
        (:RARITY_RARE
          (Appearance|SetBrushfromTexture (Variables|/Game/UI/WBP_EquipmentSlot.WBP_EquipmentSlot_C|GetRarityIcon (LocalVariables|GetLocal%20EquipmentSlot)) "/Game/Textures/Inventory/T_ItemRarity_Rare.T_ItemRarity_Rare" false))
        (:RARITY_EPIC
          (Appearance|SetBrushfromTexture (Variables|/Game/UI/WBP_EquipmentSlot.WBP_EquipmentSlot_C|GetRarityIcon (LocalVariables|GetLocal%20EquipmentSlot)) "/Game/Textures/Inventory/T_ItemRarity_Epic.T_ItemRarity_Epic" false))
        (:RARITY_LEGENDARY
          (Appearance|SetBrushfromTexture (Variables|/Game/UI/WBP_EquipmentSlot.WBP_EquipmentSlot_C|GetRarityIcon (LocalVariables|GetLocal%20EquipmentSlot)) "/Game/Textures/Inventory/T_ItemRarity_Legendary.T_ItemRarity_Legendary" false))
        (:RARITY_GODLIKE
          (Appearance|SetBrushfromTexture (Variables|/Game/UI/WBP_EquipmentSlot.WBP_EquipmentSlot_C|GetRarityIcon (LocalVariables|GetLocal%20EquipmentSlot)) "/Game/Textures/Inventory/T_ItemRarity_Godlike.T_ItemRarity_Godlike" false)))
      (Widget|SetVisibility (Variables|/Game/UI/WBP_EquipmentSlot.WBP_EquipmentSlot_C|GetRarityIcon (LocalVariables|GetLocal%20EquipmentSlot)) "HitTestInvisible")
      (if (> (Variables|/Script/TheEternalTower.EquippableItem|GetCurrentEnhancementLevel (LocalVariables|GetLocal%20Item)) 0)
        (Rendering|Components|TextRender|SetText (Variables|/Game/UI/WBP_EquipmentSlot.WBP_EquipmentSlot_C|GetEnhancementText (LocalVariables|GetLocal%20EquipmentSlot)) (Utilities|Text|FormatText "+{Enhancement Level}" (Variables|/Script/TheEternalTower.EquippableItem|GetCurrentEnhancementLevel (LocalVariables|GetLocal%20Item))))
        (else
          (Rendering|Components|TextRender|SetText (Variables|/Game/UI/WBP_EquipmentSlot.WBP_EquipmentSlot_C|GetEnhancementText (LocalVariables|GetLocal%20EquipmentSlot)) ""))))
    (:Is%20Not%20Valid
      (Variables|/Game/UI/WBP_EquipmentSlot.WBP_EquipmentSlot_C|SetHeld%20Item (LocalVariables|GetLocal%20EquipmentSlot) 0)
      (Appearance|SetBrushfromTexture (Variables|/Game/UI/WBP_EquipmentSlot.WBP_EquipmentSlot_C|GetSlotIcon (LocalVariables|GetLocal%20EquipmentSlot)) 0 false)
      (Widget|SetVisibility (Variables|/Game/UI/WBP_EquipmentSlot.WBP_EquipmentSlot_C|GetSlotIcon (LocalVariables|GetLocal%20EquipmentSlot)) "Hidden")
      (Appearance|SetBrushfromTexture (Variables|/Game/UI/WBP_EquipmentSlot.WBP_EquipmentSlot_C|GetRarityIcon (LocalVariables|GetLocal%20EquipmentSlot)) 0 false)
      (Widget|SetVisibility (Variables|/Game/UI/WBP_EquipmentSlot.WBP_EquipmentSlot_C|GetRarityIcon (LocalVariables|GetLocal%20EquipmentSlot)) "Hidden")
      (Rendering|Components|TextRender|SetText (Variables|/Game/UI/WBP_EquipmentSlot.WBP_EquipmentSlot_C|GetEnhancementText (LocalVariables|GetLocal%20EquipmentSlot)) ""))))

(fn GetMaximumHealth
  (return (+ (Variables|Default|GetMaximumHealth) (Variables|Default|GetBonusMaximumHealth))))

(fn GetMinimumPhysicalAttack
  (return (+ (Variables|Default|GetMinimumPhysicalAttackPower) (Variables|Default|GetBonusMinimumPhysicalAttackPower))))

(fn GetMaximumPhysicalAttack
  (return (+ (Variables|Default|GetMaximumPhysicalAttackPower) (Variables|Default|GetBonusMaximumPhysicalAttackPower))))

(fn GetMinimumMagicalAttack
  (return (+ (Variables|Default|GetMinimumMagicalAttackPower) (Variables|Default|GetBonusMinimumMagicalAttackPower))))

(fn GetMaximumMagicalAttack
  (return (+ (Variables|Default|GetMaximumMagicalAttackPower) (Variables|Default|GetBonusMaximumMagicalAttackPower))))

(fn GetPhysicalDefense
  (return (+ (Variables|Default|GetPhysicalDefense) (Variables|Default|GetBonusPhysicalDefense))))

(fn GetMagicalDefense
  (return (+ (Variables|Default|GetMagicalDefense) (Variables|Default|GetBonusMagicalDefense))))